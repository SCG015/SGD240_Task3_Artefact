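; BP_MapGenerator builds a square room map at BeginPlay using Wave Function Collapse over a grid of WFC_Grid cells.
; Hidden instances of each tile class supply four-direction socket lists that prune neighbouring cells' room options.
; After a random first collapse, a delayed loop propagates constraints and collapses the narrowed cell with fewest options, setting its child actor.
; A DoN fallback propagates without collapsing when no candidates exist.
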(event Custom|InitializeGrid
  ;[1 1 1] One for loop is the X, the other the Y. GridSize sets the grid size, minus 1 as we start from 0
  (for _index (range 0 (- (Variables|Default|GetDimensions) 1))
    (for _index_2 (range 0 (- (Variables|Default|GetDimensions) 1))
      ;[1 1 1] Room size X index to set the spawn transform room width apart for each room in the grid.
      (bind _returnvalue (Game|SpawnActorfromClass "/Game/WFCGen/WFC_Grid.WFC_Grid_C" (Math|Transform|MakeTransform (Math|Transform|TransformLocation (Transformation|GetActorTransform) (Math|Vector|MakeVector (Math|Conversions|ToFloat(Integer) (* _index_2 (Variables|Default|GetCellSize))) (Math|Conversions|ToFloat(Integer) (* _index (Variables|Default|GetCellSize))) 0.0)) (Transformation|GetActorRotation) "1.000000,1.000000,1.000000") "Undefined" "MultiplyWithRoot" 0 0))
      ;[1 1 1] Change from default room to random room in socket array
      (Default|BuildGrid _returnvalue (Variables|Default|GettileObjects))
      (Utilities|Array|AddUnique (Variables|Default|GetGridComponents) _returnvalue)))
  (CallFunction|CollapseFirstCell (Variables|Default|GetGridComponents))
  ;[1 1 1] Remove any collapsed cells - sort cells by their least avaialbe options and then collapse the one with the lowest value - perform a check to see if there are any cells left to collapse - if so loop back to start
  (Utilities|FlowControl|Delay 1.0 :!label _label)
  ;[1 1 1] debug
  (for _array_element 0
    (Development|PrintString (Utilities|GetDisplayName _array_element) true true "(R=1.000000,G=0.000000,B=0.310125,A=1.000000)" 0.5))
  (bind _prunedgrid (CallFunction|RemoveCollapsedCells (Variables|Default|GetGridComponents)))
  (if (> (Utilities|Array|Length _prunedgrid) 0)
    (Utilities|FlowControl|Sequence
      (:then_0
        (bind _sortedlist (CallFunction|SortbyLeastOption _prunedgrid))
        (CallFunction|CollapseCellandRemove _sortedlist)
        ;[1 1 1] debug
        (for _array_element_2 _sortedlist
          (Development|PrintString (Utilities|GetDisplayName _array_element_2) true true "(R=1.000000,G=0.866475,B=0.000000,A=1.000000)"))
        (Variables|Default|SetContinue? false :!label _label_2)
        (for _array_element_3 (Variables|Default|GetGridComponents)
          (if (not (Variables|/Game/WFCGen/WFC_Grid.WFC_Grid_C|GetisCollpased _array_element_3))
            (Variables|Default|SetContinue? true)))
        (if (Variables|Default|GetContinue?)
          (CallFunction|UpdateGeneration)
          (goto _label)))
      (:then_1
        (goto _label_3 Reset)))
    (else
      (bind _counter (Utilities|FlowControl|DoN (Variables|Default|GetUpdateWithoutCollapseStop) :!label _label_3)
        (:Exit
          (if (not (== _counter (Variables|Default|GetUpdateWithoutCollapseStop)))
            (goto _label_2)))))))

(event EventBeginPlay
  ;[1 1 1] Spawn all the rooms in the room list then get a reference for each one
  (Utilities|FlowControl|Sequence
    (:then_0
      (Utilities|Array|Clear (Variables|Default|GetTileReferenceObjects))
      (for _array_element (Variables|Default|GettileObjects)
        (bind _returnvalue (Game|SpawnActorfromClass _array_element (Math|Transform|MakeTransform "0.000000,0.000000,-500.000000" "0, 0, 0" "1.000000,1.000000,1.000000") "AlwaysSpawn" "MultiplyWithRoot" 0 0))
        (Utilities|Array|AddUnique (Variables|Default|GetTileReferenceObjects) _returnvalue)
        ;[1 1 1] Otherwise hide them and turn off collision
        (Rendering|SetActorHiddenInGame _returnvalue true)
        (Collision|SetActorEnableCollision _returnvalue false)))
    (:then_1
      ;[1 1 1] Clear array then spawn in grid
      (Utilities|Array|Clear (Variables|Default|GetGridComponents))
      (CallFunction|InitializeGrid))))

(fn ConstructionScript)

(fn CollapseFirstCell
  (params (SortedGrid :type Array%20of%20WFC%20Grid%20Object%20References))
  ;[1 1 1] Collapse a random cell that hasnt already been collapsed
  (LocalVariables|SetRandomCell%28L%29 (.OutItem (Utilities|Array|Random SortedGrid)))
  (if (not (Variables|/Game/WFCGen/WFC_Grid.WFC_Grid_C|GetisCollpased (LocalVariables|GetRandomCell%28L%29)))
    (Variables|/Game/WFCGen/WFC_Grid.WFC_Grid_C|SetisCollpased (LocalVariables|GetRandomCell%28L%29) true)
    ;[1 1 1] Make cell able to propogate
    (Variables|/Game/WFCGen/WFC_Grid.WFC_Grid_C|SetcanPropogate (LocalVariables|GetRandomCell%28L%29) true)
    ;[1 1 1] Pick a random room type from the list as the spawn room
    (LocalVariables|SetRandomTile%28L%29 (.OutItem (Utilities|Array|Random (Variables|/Game/WFCGen/WFC_Grid.WFC_Grid_C|GetRoomList (LocalVariables|GetRandomCell%28L%29)))))
    ;[1 1 1] Clear all other possible rooms then add the selected random
    (Utilities|FlowControl|Sequence
      (:then_0
        ;[1 1 1] Change the child actor to the random room
        (ChildActorComponent|SetChildActorClass (Variables|/Game/WFCGen/WFC_Grid.WFC_Grid_C|GetChildActor (LocalVariables|GetRandomCell%28L%29)) (LocalVariables|GetRandomTile%28L%29)))
      (:then_1
        (Utilities|Array|Clear (Variables|/Game/WFCGen/WFC_Grid.WFC_Grid_C|GetRoomList (LocalVariables|GetRandomCell%28L%29))))
      (:then_2
        (Utilities|Array|Add (Variables|/Game/WFCGen/WFC_Grid.WFC_Grid_C|GetRoomList (LocalVariables|GetRandomCell%28L%29)) (LocalVariables|GetRandomTile%28L%29))))))

(fn RemoveCollapsedCells
  (params (GridComponents :type Array%20of%20WFC%20Grid%20Object%20References))
  (bind _output_get (LocalVariables|SetTempGrid%28L%29 GridComponents))
  (bind _arrayelement (Utilities|Array|ReverseforEachLoop _output_get)
    (:LoopBody
      ;[1 1 1] Dont include cells that have all their possibilties open
      (if (== (Utilities|Array|LastIndex (Variables|/Game/WFCGen/WFC_Grid.WFC_Grid_C|GetRoomList _arrayelement)) (Utilities|Array|LastIndex (Variables|Default|GettileObjects)))
        (Utilities|Array|RemoveItem (LocalVariables|GetTempGrid%28L%29) _arrayelement)
        (else
          ;[1 1 1] Remove already collapsed cells
          (if (Variables|/Game/WFCGen/WFC_Grid.WFC_Grid_C|GetisCollpased _arrayelement)
            (Utilities|Array|RemoveItem (LocalVariables|GetTempGrid%28L%29) 0)
            (else
              ;[1 1 1] Remove cells with no options and arent collapsed
              (if (not (> (Utilities|Array|Length (Variables|/Game/WFCGen/WFC_Grid.WFC_Grid_C|GetRoomList _arrayelement)) 0))
                (Utilities|Array|RemoveItem (LocalVariables|GetTempGrid%28L%29) _arrayelement)))))))
    (:Completed
      (return (LocalVariables|GetTempGrid%28L%29)))))

(fn SortbyLeastOption
  (params (GridList :type Array%20of%20WFC%20Grid%20Object%20References))
  (for (_array_element _array_index) GridList
    (LocalVariables|SetCurrentCell _array_element)
    (LocalVariables|SetCurrentArrayStepper _array_index)
    (if (Utilities|Array|IsValidIndex (LocalVariables|GetSortingList%28L%29))
      (LocalVariables|SetCurrentOptionsLength (Utilities|Array|Length (Variables|/Game/WFCGen/WFC_Grid.WFC_Grid_C|GetRoomList (LocalVariables|GetCurrentCell))))
      (while (and (< (LocalVariables|GetCurrentOptionsLength) (Utilities|Array|Length (Variables|/Game/WFCGen/WFC_Grid.WFC_Grid_C|GetRoomList (Utilities|Array|Get(acopy) (LocalVariables|GetSortingList%28L%29) (+ (LocalVariables|GetCurrentArrayStepper) (Math|Integer|SelectInt -1 0 (> (LocalVariables|GetCurrentArrayStepper) 0))))))) (!= (LocalVariables|GetCurrentArrayStepper) 0))
        (LocalVariables|SetCurrentArrayStepper (+ (LocalVariables|GetCurrentArrayStepper) -1)))
      (Utilities|Array|Insert (LocalVariables|GetSortingList%28L%29) (LocalVariables|GetCurrentCell) (LocalVariables|GetCurrentArrayStepper))
      (else
        (Utilities|Array|Add (LocalVariables|GetSortingList%28L%29) (LocalVariables|GetCurrentCell)))))
  (return (LocalVariables|GetSortingList%28L%29)))

(fn CollapseCellandRemove
  (params (SortedGridList :type Array%20of%20WFC%20Grid%20Object%20References))
  (bind _output (Utilities|Array|Get(acopy) SortedGridList))
  (bind _roomlist (Variables|/Game/WFCGen/WFC_Grid.WFC_Grid_C|GetRoomList _output))
  ;[1 1 1] From the sorted list get first entry and check if that target has collapsed - set to collapsed and can propogate - get a random room type from the list and change the cell to that room type
  (if (not (Variables|/Game/WFCGen/WFC_Grid.WFC_Grid_C|GetisCollpased _output))
    (Variables|/Game/WFCGen/WFC_Grid.WFC_Grid_C|SetisCollpased _output true)
    (Variables|/Game/WFCGen/WFC_Grid.WFC_Grid_C|SetcanPropogate _output true)
    (LocalVariables|SetRandomTile%28L%29 (.OutItem (Utilities|Array|Random (Variables|/Game/WFCGen/WFC_Grid.WFC_Grid_C|GetRoomList _output))))
    (Utilities|FlowControl|Sequence
      (:then_0
        (ChildActorComponent|SetChildActorClass (Variables|/Game/WFCGen/WFC_Grid.WFC_Grid_C|GetChildActor _output) (LocalVariables|GetRandomTile%28L%29)))
      (:then_1
        (Utilities|Array|Clear _roomlist))
      (:then_2
        (Utilities|Array|Add _roomlist (LocalVariables|GetRandomTile%28L%29))))))

(fn UpdateGeneration
  ;[1 1 1] Generate Grid for X and Y
  (for _index (range 0 (- (Variables|Default|GetDimensions) 1))
    (LocalVariables|SetYGridCoord%28L%29 _index)
    (for _index_2 (range 0 (- (Variables|Default|GetDimensions) 1))
      (LocalVariables|SetXGridCoord%28L%29 _index_2)
      ;[1 1 1] Build index of cell coordiantes
      (LocalVariables|SetIndex%28L%29 (+ (LocalVariables|GetXGridCoord%28L%29) (* (LocalVariables|GetYGridCoord%28L%29) (Variables|Default|GetDimensions))))
      ;[1 1 1] If the current cell can propogate
      (if (Variables|/Game/WFCGen/WFC_Grid.WFC_Grid_C|GetcanPropogate (Utilities|Array|Get(acopy) (Variables|Default|GetGridComponents) (LocalVariables|GetIndex%28L%29)))
        (Utilities|FlowControl|Sequence
          (:then_0
            (Utilities|FlowControl|Sequence
              (:then_0
                ;[1 1 1] Check if in top row
                (if (> (LocalVariables|GetYGridCoord%28L%29) 0)
                  (CallFunction|CompareCells (LocalVariables|GetIndex%28L%29) (+ (LocalVariables|GetXGridCoord%28L%29) (* (+ (LocalVariables|GetYGridCoord%28L%29) -1) (Variables|Default|GetDimensions))) "NewEnumerator0")))
              (:then_1
                ;[1 1 1] Check if in right column
                (if (< (LocalVariables|GetXGridCoord%28L%29) (- (Variables|Default|GetDimensions) 1))
                  (CallFunction|CompareCells (LocalVariables|GetIndex%28L%29) (+ (+ (LocalVariables|GetXGridCoord%28L%29) 1) (* (LocalVariables|GetYGridCoord%28L%29) (Variables|Default|GetDimensions))) "NewEnumerator1")))
              (:then_2
                ;[1 1 1] Check if in bottom row
                (if (< (LocalVariables|GetYGridCoord%28L%29) (- (Variables|Default|GetDimensions) 1))
                  (CallFunction|CompareCells (LocalVariables|GetIndex%28L%29) (+ (LocalVariables|GetXGridCoord%28L%29) (* (+ (LocalVariables|GetYGridCoord%28L%29) 1) (Variables|Default|GetDimensions))) "NewEnumerator2")))
              (:then_3
                ;[1 1 1] Check if in left column
                (if (> (LocalVariables|GetXGridCoord%28L%29) 0)
                  (CallFunction|CompareCells (LocalVariables|GetIndex%28L%29) (+ (+ (LocalVariables|GetXGridCoord%28L%29) -1) (* (LocalVariables|GetYGridCoord%28L%29) (Variables|Default|GetDimensions))) "NewEnumerator3")))))
          (:then_1
            ;[1 1 1] Then set cell propogation to false
            (Variables|/Game/WFCGen/WFC_Grid.WFC_Grid_C|SetcanPropogate (Utilities|Array|Get(acopy) (Variables|Default|GetGridComponents) (LocalVariables|GetIndex%28L%29)) false))))))
  (return))

(fn CompareCells
  (params (PrimaryCellIndex :type Integer) (AdjacentCellIndex :type Integer) (Direction :type EDirection%20Enum :default "NewEnumerator0"))
  (bind _gridcomponents (Variables|Default|GetGridComponents))
  (bind _output (Utilities|Array|Get(acopy) _gridcomponents AdjacentCellIndex))
  (bind _roomlist (Variables|/Game/WFCGen/WFC_Grid.WFC_Grid_C|GetRoomList _output))
  ;[1 1 1] If the neighbour appears in the room list dump neighbours in that cells direction into a list
  (bind _arrayelement (Utilities|Array|ReverseforEachLoop (Variables|Default|GetTileReferenceObjects))
    (:LoopBody
      (if (Utilities|Array|ContainsItem (Variables|/Game/WFCGen/WFC_Grid.WFC_Grid_C|GetRoomList (Utilities|Array|Get(acopy) (Variables|Default|GetGridComponents) PrimaryCellIndex)) (Utilities|GetClass _arrayelement))
        ;[1 1 1] Dump all possible adjacents into a list
        (Utilities|Set|AddItems (LocalVariables|GettempDumpList%28L%29) (Utilities|Select :Index Direction :NewEnumerator0 (Variables|/Game/WFCGen/WFC_RoomTemplate.WFC_RoomTemplate_C|GetSocketUp _arrayelement) :NewEnumerator1 (Variables|/Game/WFCGen/WFC_RoomTemplate.WFC_RoomTemplate_C|GetSocketRight _arrayelement) :NewEnumerator2 (Variables|/Game/WFCGen/WFC_RoomTemplate.WFC_RoomTemplate_C|GetSocketDown _arrayelement) :NewEnumerator3 (Variables|/Game/WFCGen/WFC_RoomTemplate.WFC_RoomTemplate_C|GetSocketLeft _arrayelement)))))
    (:Completed
      ;[1 1 1] Remove options of adjacent cells  that arent in the
      (bind _arrayelement_2 (Utilities|Array|ReverseforEachLoop _roomlist)
        (:LoopBody
          (if (not (Utilities|Set|Contains (LocalVariables|GettempDumpList%28L%29) _arrayelement_2))
            (bind _returnvalue (Utilities|Array|RemoveItem _roomlist _arrayelement_2))
            ;[1 1 1] If anything removed from the options set ready to propogate
            (if _returnvalue
              (Utilities|FlowControl|DoOnce false
                (:Completed
                  (Variables|/Game/WFCGen/WFC_Grid.WFC_Grid_C|SetcanPropogate (Utilities|Array|Get(acopy) (Variables|Default|GetGridComponents) AdjacentCellIndex) true))))))))))